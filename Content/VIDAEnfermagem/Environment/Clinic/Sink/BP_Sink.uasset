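; Clinic sink for a nursing simulation, where Leap hands wash in the trigger volume.
; Overlap toggles the water and fades its sound.
; In the FSM's Put on Glasses or Wash Hands states, three-second timers mark each hand washed; once both are, hand exit logs to the report and calls HandsWashed.
; Exit clears timers by outdated Portuguese function names, so early withdrawal does not cancel washing.
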(event `self.ReceiveBeginPlay`
  (`AudioComponent.Stop` (`self.aguasom`)))

(event `self.WashingTrigger.OnComponentBeginOverlap`
  (params (OverlappedComponent :type "PrimitiveComponent Object Reference") (OtherActor :type "Actor Object Reference") (OtherComp :type "PrimitiveComponent Object Reference") (OtherBodyIndex :type Integer) (bFromSweep :type Boolean) (SweepResult :type "HitResult Structure (by ref)"))
  (`SceneComponent.SetVisibility` (`self.fonteAgua`) true true)
  (`AudioComponent.FadeIn` (`self.aguasom`) 0.3 1.0 (`KismetMathLibrary.Conv_IntToDouble` (`KismetMathLibrary.RandomInteger` 9)))
  (switch `/Game/VIDAEnfermagem/Core/E_ProcedureState` (`/Game/VIDAEnfermagem/Core/BP_ProcedureFSM.State` (`self.FSM`))
    (:`NewEnumerator0`
      _)
    (:`NewEnumerator1`
      _))
  (bind _asbp_custom_leap_low_poly_hand (cast `/Game/VIDAEnfermagem/Core/Leap/BP_CustomLeapLowPolyHand` OtherActor))
  (`|ExecutionSequence`
    (:`then_0`
      (if (and (== (`/Game/VIDAEnfermagem/Core/Leap/BP_CustomLeapLowPolyHand.Right` _asbp_custom_leap_low_poly_hand) OtherComp) (not (`self.bRightWashed`)))
        (`KismetSystemLibrary.K2_SetTimer` self "WashRightHand" 3.0)))
    (:`then_1`
      (if (and (== (`/Game/VIDAEnfermagem/Core/Leap/BP_CustomLeapLowPolyHand.Left` _asbp_custom_leap_low_poly_hand) OtherComp) (not (`self.bLeftWashed`)))
        (`KismetSystemLibrary.K2_SetTimer` self "WashLeftHand" 3.0)))))

(event `self.WashingTrigger.OnComponentEndOverlap`
  (params (OverlappedComponent :type "PrimitiveComponent Object Reference") (OtherActor :type "Actor Object Reference") (OtherComp :type "PrimitiveComponent Object Reference") (OtherBodyIndex :type Integer))
  (`SceneComponent.SetVisibility` (`self.fonteAgua`) false true)
  (bind _asbp_custom_leap_low_poly_hand (cast `/Game/VIDAEnfermagem/Core/Leap/BP_CustomLeapLowPolyHand` OtherActor))
  (`AudioComponent.FadeOut` (`self.aguasom`) 0.5 0.0)
  (`|ExecutionSequence`
    (:`then_0`
      (if (== (`/Game/VIDAEnfermagem/Core/Leap/BP_CustomLeapLowPolyHand.Right` _asbp_custom_leap_low_poly_hand) OtherComp)
        (`KismetSystemLibrary.K2_ClearTimer` self "HigienizarMãoDireita")
        (if (and (`self.bRightWashed`) (`self.bLeftWashed`)) :!label _label
          (`KismetSystemLibrary.PrintString` "Higienização completa!")
          (`/Game/VIDAEnfermagem/Core/WriteText.EscreveRelatorio` "Higienizou mãos")
          (`/Game/VIDAEnfermagem/Core/BP_ProcedureFSM.HandsWashed` (`self.FSM`))
          (set `self.bRightWashed` false)
          (set `self.bLeftWashed` false))))
    (:`then_1`
      (if (== (`/Game/VIDAEnfermagem/Core/Leap/BP_CustomLeapLowPolyHand.Left` _asbp_custom_leap_low_poly_hand) OtherComp)
        (`KismetSystemLibrary.K2_ClearTimer` self "HigienizarMãoEsquerda")
        (goto _label)))))

(fn `UserConstructionScript`)

(fn `WashLeftHand`
  (set `self.bLeftWashed` true)
  (`KismetSystemLibrary.PrintString` "Left hand washed."))

(fn `WashRightHand`
  (set `self.bRightWashed` true)
  (`KismetSystemLibrary.PrintString` "Right hand washed."))