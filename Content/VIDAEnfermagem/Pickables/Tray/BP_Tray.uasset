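; Nursing-simulation tray that receives blood-collection items (tourniquet, syringe, tube, wet and dry cotton, needle) carried by Leap or floating hands.
; On box overlap, an item's first placement releases it from the hand, snaps it to its preset slot, saves that as its default transform and logs a report entry.
; Items already placed only toggle their tray-trigger flag on overlap begin and end.
; The tray itself overrides picking to disabled.
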(event `self.ReceiveBeginPlay`
  (`self.setup`))

(event `self.ReceiveTick`
  (params (DeltaSeconds :type "Float (single-precision)")))

(event `self.Box.OnComponentBeginOverlap`
  (params (OverlappedComponent :type "PrimitiveComponent Object Reference") (OtherActor :type "Actor Object Reference") (OtherComp :type "PrimitiveComponent Object Reference") (OtherBodyIndex :type Integer) (bFromSweep :type Boolean) (SweepResult :type "HitResult Structure (by ref)"))
  (bind _keeprelative (`self.KeepRelative`))
  (bind _transformpadraoagulha (`self.TransformPadraoAgulha`))
  (bind _transformpadraogarrote (`self.TransformPadraoGarrote`))
  (bind _transformpadraointermediario (`self.TransformPadraoIntermediario`))
  (bind _transformpadraocoletor (`self.TransformPadraoColetor`))
  (bind _transformpadraoalgodaoantisseptico (`self.TransformPadraoAlgodaoAntisseptico`))
  (bind _keeprelative_2 (`self.KeepRelative`))
  (bind _keeprelative_3 (`self.KeepRelative`))
  (bind _keeprelative_4 (`self.KeepRelative`))
  (bind _keeprelative_5 (`self.KeepRelative`))
  (bind _keeprelative_6 (`self.KeepRelative`))
  (bind _transformpadraoalgodaoseco (`self.TransformPadraoAlgodaoSeco`))
  (bind _returnvalue (`self.GetAttachParentActor` (`ActorComponent.GetOwner` (`Actor.RootComponent` OtherActor))))
  (cast `/Game/VIDAEnfermagem/Core/Leap/BP_CustomLeapLowPolyHand` _returnvalue
    (:`then`
      _)
    (:`CastFailed`
      (cast `/Game/VIDAEnfermagem/Characters/Player/BP_FloatingHands` _returnvalue)))
  (bind _asbp_tourniquet_buckle (cast `/Game/VIDAEnfermagem/Pickables/TourniquetBuckle/BP_TourniquetBuckle` OtherActor)
    (:`then`
      (if (`/Game/VIDAEnfermagem/Core/BP_PickableObject.FoiColocadoNaBandeja` _asbp_tourniquet_buckle)
        (set `/Game/VIDAEnfermagem/Core/BP_PickableObject.triggerBandeja` true _asbp_tourniquet_buckle)
        (else
          (`self.SoltarDaMão_0` _asbp_tourniquet_buckle)
          (`self.K2_AttachToActor` _asbp_tourniquet_buckle self "None" _keeprelative _keeprelative _keeprelative true)
          (`self.K2_SetActorRelativeTransform` _asbp_tourniquet_buckle _transformpadraogarrote false false)
          (set `/Game/VIDAEnfermagem/Core/BP_PickableObject.transformPadrao` _transformpadraogarrote _asbp_tourniquet_buckle)
          (set `/Game/VIDAEnfermagem/Core/BP_PickableObject.FoiColocadoNaBandeja` true _asbp_tourniquet_buckle)
          (`/Game/VIDAEnfermagem/Core/WriteText.EscreveRelatorio` "Colocou  Garrote na Bandeja"))))
    (:`CastFailed`
      (bind _asbp_syringe (cast `/Game/VIDAEnfermagem/Pickables/Syringe/BP_Syringe` OtherActor)
        (:`then`
          (if (`/Game/VIDAEnfermagem/Core/BP_PickableObject.FoiColocadoNaBandeja` _asbp_syringe)
            (set `/Game/VIDAEnfermagem/Core/BP_PickableObject.triggerBandeja` true _asbp_syringe)
            (else
              (`self.SoltarDaMão_0` _asbp_syringe)
              (`self.K2_AttachToActor` _asbp_syringe self "None" _keeprelative_3 _keeprelative_3 _keeprelative_3 true)
              (`self.K2_SetActorRelativeTransform` _asbp_syringe _transformpadraointermediario false false)
              (set `/Game/VIDAEnfermagem/Core/BP_PickableObject.transformPadrao` _transformpadraointermediario _asbp_syringe)
              (set `/Game/VIDAEnfermagem/Core/BP_PickableObject.FoiColocadoNaBandeja` true _asbp_syringe)
              (`/Game/VIDAEnfermagem/Core/WriteText.EscreveRelatorio` "Colocou  Intermediario na Bandeja"))))
        (:`CastFailed`
          (bind _asbp_collection_tube (cast `/Game/VIDAEnfermagem/Pickables/CollectionTube/BP_CollectionTube` OtherActor)
            (:`then`
              (if (`/Game/VIDAEnfermagem/Core/BP_PickableObject.FoiColocadoNaBandeja` _asbp_collection_tube)
                (set `/Game/VIDAEnfermagem/Core/BP_PickableObject.triggerBandeja` true _asbp_collection_tube)
                (else
                  (`self.SoltarDaMão_0` _asbp_collection_tube)
                  (`self.K2_AttachToActor` _asbp_collection_tube self "None" _keeprelative_5 _keeprelative_5 _keeprelative_5 true)
                  (`self.K2_SetActorRelativeTransform` _asbp_collection_tube _transformpadraocoletor false false)
                  (set `/Game/VIDAEnfermagem/Core/BP_PickableObject.transformPadrao` _transformpadraocoletor _asbp_collection_tube)
                  (set `/Game/VIDAEnfermagem/Core/BP_PickableObject.FoiColocadoNaBandeja` true _asbp_collection_tube)
                  (`/Game/VIDAEnfermagem/Core/WriteText.EscreveRelatorio` "Colocou  Coletor na Bandeja"))))
            (:`CastFailed`
              (bind _asbp_cotton_wet (cast `/Game/VIDAEnfermagem/Pickables/Cotton/BP_Cotton_Wet` OtherActor)
                (:`then`
                  (if (`/Game/VIDAEnfermagem/Core/BP_PickableObject.FoiColocadoNaBandeja` _asbp_cotton_wet)
                    (set `/Game/VIDAEnfermagem/Core/BP_PickableObject.triggerBandeja` true _asbp_cotton_wet)
                    (else
                      (`self.SoltarDaMão_0` _asbp_cotton_wet)
                      (`self.K2_AttachToActor` _asbp_cotton_wet self "None" _keeprelative_6 _keeprelative_6 _keeprelative_6 true)
                      (`self.K2_SetActorRelativeTransform` _asbp_cotton_wet _transformpadraoalgodaoantisseptico false false)
                      (set `/Game/VIDAEnfermagem/Core/BP_PickableObject.transformPadrao` _transformpadraoalgodaoantisseptico _asbp_cotton_wet)
                      (set `/Game/VIDAEnfermagem/Core/BP_PickableObject.FoiColocadoNaBandeja` true _asbp_cotton_wet)
                      (`/Game/VIDAEnfermagem/Core/WriteText.EscreveRelatorio` "Colocou  Algodão Antisséptic na Bandeja"))))
                (:`CastFailed`
                  (bind _asbp_cotton_dry (cast `/Game/VIDAEnfermagem/Pickables/Cotton/BP_Cotton_Dry` OtherActor)
                    (:`then`
                      (if (`/Game/VIDAEnfermagem/Core/BP_PickableObject.FoiColocadoNaBandeja` _asbp_cotton_dry)
                        (set `/Game/VIDAEnfermagem/Core/BP_PickableObject.triggerBandeja` true _asbp_cotton_dry)
                        (else
                          (`self.SoltarDaMão_0` _asbp_cotton_dry)
                          (`self.K2_AttachToActor` _asbp_cotton_dry self "None" _keeprelative_4 _keeprelative_4 _keeprelative_4 true)
                          (`self.K2_SetActorRelativeTransform` _asbp_cotton_dry _transformpadraoalgodaoseco false false)
                          (set `/Game/VIDAEnfermagem/Core/BP_PickableObject.transformPadrao` _transformpadraoalgodaoseco _asbp_cotton_dry)
                          (set `/Game/VIDAEnfermagem/Core/BP_PickableObject.FoiColocadoNaBandeja` true _asbp_cotton_dry)
                          (`/Game/VIDAEnfermagem/Core/WriteText.EscreveRelatorio` "Colocou  Algodão Seco na Bandeja"))))
                    (:`CastFailed`
                      (bind _asbp_needle (cast `/Game/VIDAEnfermagem/Pickables/Syringe/BP_Needle` OtherActor))
                      (if (`/Game/VIDAEnfermagem/Core/BP_PickableObject.FoiColocadoNaBandeja` _asbp_needle)
                        (set `/Game/VIDAEnfermagem/Core/BP_PickableObject.triggerBandeja` true _asbp_needle)
                        (else
                          (`self.SoltarDaMão_0` _asbp_needle)
                          (`self.K2_AttachToActor` _asbp_needle self "None" _keeprelative_2 _keeprelative_2 _keeprelative_2 true)
                          (`self.K2_SetActorRelativeTransform` _asbp_needle _transformpadraoagulha false false)
                          (set `/Game/VIDAEnfermagem/Core/BP_PickableObject.transformPadrao` _transformpadraoagulha _asbp_needle)
                          (set `/Game/VIDAEnfermagem/Core/BP_PickableObject.FoiColocadoNaBandeja` true _asbp_needle)
                          (`/Game/VIDAEnfermagem/Core/WriteText.EscreveRelatorio` "Colocou  Agulha na Bandeja"))))))))))))))

(event `self.Box.OnComponentEndOverlap`
  (params (OverlappedComponent :type "PrimitiveComponent Object Reference") (OtherActor :type "Actor Object Reference") (OtherComp :type "PrimitiveComponent Object Reference") (OtherBodyIndex :type Integer))
  (bind _asbp_pickable_object (cast `/Game/VIDAEnfermagem/Core/BP_PickableObject` OtherActor))
  (set `/Game/VIDAEnfermagem/Core/BP_PickableObject.triggerBandeja` false _asbp_pickable_object))

(fn `IsPickingEnabled`
  (returns (pegarAtivado :type Boolean))
  (`parent.IsPickingEnabled`)
  (return false))

(fn `SetarReferencias`
  (bind _returnvalue (`KismetSystemLibrary.IsValid` (`self.JogadorReferencia`)))
  (while (not (`self.ReferenciasSetadas`))
    (if (not _returnvalue)
      (bind _outactors (`GameplayStatics.GetAllActorsOfClass` "/Game/VIDAEnfermagem/Characters/Player/BP_FloatingHands.BP_FloatingHands_C"))
      (set `self.JogadorReferencia` (`|GetArrayItem` _outactors)))
    (set `self.ReferenciasSetadas` _returnvalue)))

(fn `setup`
  (bind (_transformpadrao_location _transformpadrao_rotation _transformpadrao_scale) (`KismetMathLibrary.BreakTransform` (`self.transformPadrao`)))
  (`parent.ReceiveBeginPlay`)
  (set `self.transformMaoDireita` (`KismetMathLibrary.MakeTransform` (-22.48 16.57 14.89) (struct :`Pitch` 27.440001 :`Yaw` 104.519997 :`Roll` -8.91) _transformpadrao_scale))
  (set `self.transformMaoEsquerda` (`KismetMathLibrary.MakeTransform` (20.741327 -23.360912 -5.805843) (struct :`Yaw` 97.186996 :`Roll` 158.389999) _transformpadrao_scale))
  (`self.SetarReferencias`))

(fn `SoltarDaMão_0`
  (params (ObjetoPegavel :type "/Game/VIDAEnfermagem/Core/BP_PickableObject Object Reference"))
  (bind _jogadorreferencia (`self.JogadorReferencia`))
  (if (`/Game/VIDAEnfermagem/Characters/Player/BP_FloatingHands.PegandoDireita` _jogadorreferencia)
    (if (`KismetStringLibrary.EqualEqual_StrStr` (`KismetSystemLibrary.GetDisplayName` (`/Game/VIDAEnfermagem/Characters/Player/BP_FloatingHands.ObjetoAnexadoDireita` _jogadorreferencia)) (`KismetSystemLibrary.GetDisplayName` ObjetoPegavel))
      (`/Game/VIDAEnfermagem/Characters/Player/BP_FloatingHands.Soltar_D` _jogadorreferencia)
      (else
        (if (`/Game/VIDAEnfermagem/Characters/Player/BP_FloatingHands.PegandoEsquerda` _jogadorreferencia) :!label _label
          (if (`KismetStringLibrary.EqualEqual_StrStr` (`KismetSystemLibrary.GetDisplayName` ObjetoPegavel) (`KismetSystemLibrary.GetDisplayName` (`/Game/VIDAEnfermagem/Characters/Player/BP_FloatingHands.ObjetoAnexadoEsquerda` _jogadorreferencia)))
            (`/Game/VIDAEnfermagem/Characters/Player/BP_FloatingHands.Soltar_E` _jogadorreferencia)))))
    (else
      (goto _label))))

(fn `UserConstructionScript`)