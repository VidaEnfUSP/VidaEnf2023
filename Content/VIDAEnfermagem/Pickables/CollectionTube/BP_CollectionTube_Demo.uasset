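; Pickable blood collection tube for the nursing demo, grabbable only once the game mode has started.
; Overlapping a syringe that is in the arm snaps a non-full tube onto it, starting collection if in the vein.
; Tick grows the blood mesh's Z scale until full, then counts up/down orientation changes, flagging homogenization after ten full inversions.
; Setup sets hand grip transforms and finds the patient and syringe actors.
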(event `self.ReceiveBeginPlay`
  (`self.setup`))

(event `self.ColisãoDoColetor.OnComponentBeginOverlap`
  (params (OverlappedComponent :type "PrimitiveComponent Object Reference") (OtherActor :type "Actor Object Reference") (OtherComp :type "PrimitiveComponent Object Reference") (OtherBodyIndex :type Integer) (bFromSweep :type Boolean) (SweepResult :type "HitResult Structure (by ref)"))
  (`self.AnexarNoIntermediarioSeNaVeia` OtherActor OtherComp))

(event `self.ColisãoDoColetor.OnComponentEndOverlap`
  (params (OverlappedComponent :type "PrimitiveComponent Object Reference") (OtherActor :type "Actor Object Reference") (OtherComp :type "PrimitiveComponent Object Reference") (OtherBodyIndex :type Integer))
  (if (`KismetStringLibrary.EqualEqual_StrStr` "CorpoDoIntermediário" (`KismetSystemLibrary.GetObjectName` OtherComp))
    (set `self.coletando` false)))

(event `self.ReceiveTick`
  (params (DeltaSeconds :type "Float (single-precision)"))
  (`parent.ReceiveTick` DeltaSeconds)
  (`self.EscalarSangueSeColetando`)
  (if (`self.cheio`)
    (`self.SetCimaBaixo`))
  (if (`self.noIntermediário`)
    (cast `/Game/VIDAEnfermagem/Pickables/Syringe/BP_Syringe` (`ActorComponent.GetOwner` (`SceneComponent.GetAttachParent` (`self.RootComponent`)))
      (:`CastFailed`
        (bind _output_get (set `self.noIntermediário` false))
        (set `/Game/VIDAEnfermagem/Pickables/Syringe/BP_Syringe_Demo.coletorAnexado` _output_get (`self.intermediario`))))))

(fn `AnexarNoIntermediarioSeNaVeia`
  (params (Actor :type "Actor Object Reference") (Componet :type "Object Object Reference"))
  (if (not (`self.cheio`))
    (bind _asbp_syringe_demo (cast `/Game/VIDAEnfermagem/Pickables/Syringe/BP_Syringe_Demo` Actor))
    (if (`/Game/VIDAEnfermagem/Pickables/Syringe/BP_Syringe_Demo.noBraço` _asbp_syringe_demo)
      (`self.soltarDaMão`)
      (`SceneComponent.K2_AttachToComponent` (`self.RootComponent`) (`Actor.RootComponent` (`self.intermediario`)) "None" "KeepRelative" "KeepRelative" "KeepRelative" true)
      (`self.K2_SetActorTransform` (`self.GetTransform` Actor))
      (if (`/Game/VIDAEnfermagem/Pickables/Syringe/BP_Syringe_Demo.naVeia` _asbp_syringe_demo)
        (set `self.coletando` true)
        (set `self.procedimentoEmProgresso` true))
      (set `self.noIntermediário` true)
      (set `/Game/VIDAEnfermagem/Pickables/Syringe/BP_Syringe_Demo.coletorAnexado` true _asbp_syringe_demo)
      (return))
    (else
      (return))))

(fn `EscalarSangueSeColetando`
  (returns (coletorCheio :type Boolean))
  (bind _sangue (`self.Sangue`))
  (bind _relativescale3d (`SceneComponent.RelativeScale3D` _sangue))
  (if (`self.coletando`)
    (`/Engine/EditorBlueprintResources/StandardMacros.CompareFloat` (.z _relativescale3d) 0.6
      (:`>`
        (bind _output_get (set `self.coletando` false :!label _label))
        (set `self.cheio` true)
        (`/Game/VIDAEnfermagem/Core/WriteText.EscreveRelatorio` "Coletor Cheio")
        (return _output_get))
      (:`==`
        (goto _label))
      (:`<`
        (`SceneComponent.SetRelativeScale3D` _sangue (+ _relativescale3d (`KismetMathLibrary.MakeVector` 0.0 0.0 (`self.velocidadeSangue`))))))))

(fn `IsPickingEnabled`
  (returns (pegarAtivado :type Boolean))
  (return (`/Game/VIDAEnfermagem/Core/Demo_Gamemode.Começou` (cast `/Game/VIDAEnfermagem/Core/Demo_Gamemode` (`GameplayStatics.GetGameMode`) :!pure true))))

(fn `SetarReferencias`
  (bind _returnvalue (`KismetSystemLibrary.IsValid` (`self.paciente`)))
  (bind _returnvalue_2 (`KismetSystemLibrary.IsValid` (`self.intermediario`)))
  (while (not (`self.ReferenciasSetadas`))
    (if (not _returnvalue)
      (bind _outactors (`GameplayStatics.GetAllActorsOfClass` "/Game/VIDAEnfermagem/Characters/Patient/BP_Patient_Demo.BP_Patient_Demo_C"))
      (set `self.paciente` (`|GetArrayItem` _outactors)))
    (if (not _returnvalue_2)
      (bind _outactors_2 (`GameplayStatics.GetAllActorsOfClass` "/Game/VIDAEnfermagem/Pickables/Syringe/BP_Syringe_Demo.BP_Syringe_Demo_C"))
      (set `self.intermediario` (`|GetArrayItem` _outactors_2)))
    (set `self.ReferenciasSetadas` (and _returnvalue _returnvalue_2))))

(fn `SetCimaBaixo`
  (locals (semiViradas :type "Float (double-precision)"))
  (bind _z (.z (`KismetMathLibrary.Conv_RotatorToVector` (`SceneComponent.K2_GetComponentRotation` (`self.GeometryCache`)))))
  (set `self.posicaoAnterior` (`self.novaPosicao`))
  (if (>= _z 0.75)
    (set `self.novaPosicao` "cima")
    (elif (<= _z -0.75)
      (set `self.novaPosicao` "baixo")
      (else
        (return))))
  (if (not (`KismetStringLibrary.EqualEqual_StrStr` (`self.posicaoAnterior`) (`self.novaPosicao`)))
    (bind _result (`/Engine/EditorBlueprintResources/StandardMacros.IncrementFloat` (`local.semiViradas`))
      (:`  `
        (bind _output_get (set `self.viradas` (`KismetMathLibrary.FFloor` (/ _result 2.0))))
        (`KismetSystemLibrary.PrintString` (`KismetStringLibrary.Conv_IntToString` _output_get))
        (if (>= _output_get 10)
          (set `self.homogeinizou` true)))))
  (return))

(fn `setup`
  (bind (_transformpadrao_location _transformpadrao_rotation _transformpadrao_scale) (`KismetMathLibrary.BreakTransform` (`self.transformPadrao`)))
  (`parent.ReceiveBeginPlay`)
  (set `self.transformMaoDireita` (`KismetMathLibrary.MakeTransform` (-11.0 4.0 8.0) (struct :`Pitch` 110.0) _transformpadrao_scale))
  (set `self.transformMaoEsquerda` (`KismetMathLibrary.MakeTransform` (12.0 -4.0 -5.0) (struct :`Pitch` -80.0) _transformpadrao_scale))
  (`self.SetarReferencias`))

(fn `SoltarDaMão_0`
  (params (In :type "/Game/VIDAEnfermagem/Characters/Player/BP_FloatingHands Object Reference"))
  (if (`/Game/VIDAEnfermagem/Characters/Player/BP_FloatingHands.PegandoDireita` In)
    (if (`KismetStringLibrary.EqualEqual_StrStr` (`KismetSystemLibrary.GetClassDisplayName` (`GameplayStatics.GetObjectClass` (`/Game/VIDAEnfermagem/Characters/Player/BP_FloatingHands.ObjetoAnexadoDireita` In))) "Coletor_C")
      (`/Game/VIDAEnfermagem/Characters/Player/BP_FloatingHands.Soltar_D` In))
    (elif (`/Game/VIDAEnfermagem/Characters/Player/BP_FloatingHands.PegandoEsquerda` In)
      (if (`KismetStringLibrary.EqualEqual_StrStr` (`KismetSystemLibrary.GetClassDisplayName` (`GameplayStatics.GetObjectClass` (`/Game/VIDAEnfermagem/Characters/Player/BP_FloatingHands.ObjetoAnexadoEsquerda` In))) "Coletor_C")
        (`/Game/VIDAEnfermagem/Characters/Player/BP_FloatingHands.Soltar_E` In)))))

(fn `UserConstructionScript`)